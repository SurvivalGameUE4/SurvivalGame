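; Choppable tree that the player fells with five presses of the Action input while inside its ActiveZone1 trigger, which toggles input.
; A dynamic wood material receives the HitLocation1 world position, and the first four hits deepen its cut through CutDepth1.
; The fifth hit hides the tree, shows the trunk and cut-trunk components, and turns on trunk physics.
; The construction script applies the same material setup with adjustable depth.
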(event `self.ReceiveBeginPlay`
  (bind _tree (`self.Tree`))
  (bind _returnvalue (`PrimitiveComponent.CreateDynamicMaterialInstance` _tree 1 (`PrimitiveComponent.GetMaterial` _tree 1)))
  (bind _output_get (set `self.WoodMat` _returnvalue))
  (`MaterialInstanceDynamic.SetVectorParameterValue` _output_get "HitLocation1" (`KismetMathLibrary.Conv_VectorToLinearColor` (`SceneComponent.K2_GetComponentLocation` (`self.HitLocation1`))))
  (`MaterialInstanceDynamic.SetScalarParameterValue` _output_get "CutDepth1" 0.0)
  (`MaterialInstanceDynamic.SetScalarParameterValue` _output_get "Displacement" 8.75)
  (set `self.Cut Depth Location 1` 8.75))

(event `self.ActiveZone1.OnComponentBeginOverlap`
  (params (OverlappedComponent :type "PrimitiveComponent Object Reference") (OtherActor :type "Actor Object Reference") (OtherComp :type "PrimitiveComponent Object Reference") (OtherBodyIndex :type Integer) (bFromSweep :type Boolean) (SweepResult :type "HitResult Structure (by ref)"))
  (if (not (`self.Hit5Recieved`))
    (`self.EnableInput` (`GameplayStatics.GetPlayerController` 0))
    (set `self.Zone1IsActive` true)
    (`KismetSystemLibrary.PrintString` "Press Action to Chop!" true true (struct :`R` 1.0 :`G` 1.0 :`A` 1.0))))

(event `self.ActiveZone1.OnComponentEndOverlap`
  (params (OverlappedComponent :type "PrimitiveComponent Object Reference") (OtherActor :type "Actor Object Reference") (OtherComp :type "PrimitiveComponent Object Reference") (OtherBodyIndex :type Integer))
  (`self.DisableInput` (`GameplayStatics.GetPlayerController` 0))
  (set `self.Zone1IsActive` false))

(event `InputAction|Action`
  (params (Key :type "Key Structure"))
  (bind _tree (`self.Tree`))
  (bind _tronc (`self.Tronc`))
  (bind _cut_depth_location_1 (`self.Cut Depth Location 1`))
  (bind _woodmat (`self.WoodMat`))
  (:`Pressed`
    (if (not (`self.Hit5Recieved`))
      (`ActorComponent.Activate` (`self.ParticleSystem`) true)
      (if (`self.Zone1IsActive`)
        (if (`self.Hit1Recieved`)
          (if (`self.Hit2Recieved`)
            (if (`self.Hit3Recieved`)
              (if (`self.Hit4Recieved`)
                (set `self.Hit5Recieved` true)
                (else
                  (`MaterialInstanceDynamic.SetScalarParameterValue` _woodmat "CutDepth1" (* 12.0 _cut_depth_location_1))
                  (set `self.Hit4Recieved` true)))
              (else
                (`MaterialInstanceDynamic.SetScalarParameterValue` _woodmat "CutDepth1" (* 6.0 _cut_depth_location_1))
                (set `self.Hit3Recieved` true)))
            (else
              (`MaterialInstanceDynamic.SetScalarParameterValue` _woodmat "CutDepth1" (* 3.0 _cut_depth_location_1))
              (set `self.Hit2Recieved` true)))
          (else
            (`MaterialInstanceDynamic.SetScalarParameterValue` _woodmat "CutDepth1" (* 1.0 _cut_depth_location_1))
            (set `self.Hit1Recieved` true)))
        (`KismetSystemLibrary.PrintString` "Chop!")
        (if (`self.Hit5Recieved`)
          (`KismetSystemLibrary.PrintString` "TIMBER!!!" true true (struct :`R` 1.0 :`A` 1.0))
          (`SceneComponent.SetVisibility` _tree false false)
          (`PrimitiveComponent.SetCollisionEnabled` _tree "NoCollision")
          (`SceneComponent.SetVisibility` _tronc true false)
          (`SceneComponent.SetVisibility` (`self.CuttingTronc`) true false)
          (`PrimitiveComponent.SetSimulatePhysics` _tronc true))))))

(fn `UserConstructionScript`
  (bind _tree (`self.Tree`))
  (bind _cut_depth_location_1 (`self.Cut Depth Location 1`))
  (bind _returnvalue (`PrimitiveComponent.CreateDynamicMaterialInstance` _tree 1 (`PrimitiveComponent.GetMaterial` _tree 1)))
  (bind _output_get (set `self.WoodMat` _returnvalue))
  (`MaterialInstanceDynamic.SetVectorParameterValue` _output_get "HitLocation1" (`KismetMathLibrary.Conv_VectorToLinearColor` (`SceneComponent.K2_GetComponentLocation` (`self.HitLocation1`))))
  (`MaterialInstanceDynamic.SetScalarParameterValue` _output_get "Displacement" (* _cut_depth_location_1 1.75))
  (`MaterialInstanceDynamic.SetScalarParameterValue` _output_get "CutDepth1" (* _cut_depth_location_1 (`self.CDInfluence 1`))))