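; Campfire actor with a flickering point light and proximity-based input for the survival character.
; A timeline started at BeginPlay drives the light intensity.
; A box overlap with BP_SurvivalCharacter enables or disables the actor's input and sets an Overlap flag.
; Disconnected logic, which never runs, would toggle two widgets as an inventory screen, switching character input, input mode and mouse cursor.
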(event `self.ReceiveBeginPlay`
  ;[1 1 1] Ligth Variation
  (bind (_direction _intensity) (`Timeline|Light`)
    (:`Update`
      (`LightComponent.SetIntensity` (`self.PointLight`) (* _intensity 6000.0)))))

(event `self.Box.OnComponentBeginOverlap`
  (params (OverlappedComponent :type "PrimitiveComponent Object Reference") (OtherActor :type "Actor Object Reference") (OtherComp :type "PrimitiveComponent Object Reference") (OtherBodyIndex :type Integer) (bFromSweep :type Boolean) (SweepResult :type "HitResult Structure (by ref)"))
  ;[1 1 1] Detection de la collision
  (cast `/Game/character/ThirdPersonBP/Blueprints/BP_SurvivalCharacter` OtherActor)
  (`self.EnableInput` (`GameplayStatics.GetPlayerController` 0))
  (set `self.Overlap` true))

(event `self.Box.OnComponentEndOverlap`
  (params (OverlappedComponent :type "PrimitiveComponent Object Reference") (OtherActor :type "Actor Object Reference") (OtherComp :type "PrimitiveComponent Object Reference") (OtherBodyIndex :type Integer))
  ;[1 1 1] Detection de la collision
  (cast `/Game/character/ThirdPersonBP/Blueprints/BP_SurvivalCharacter` OtherActor)
  (`self.DisableInput` (`GameplayStatics.GetPlayerController` 0))
  (set `self.Overlap` false))

(event `InputAction|Use`
  (params (Key :type "Key Structure")))

(fn `UserConstructionScript`)