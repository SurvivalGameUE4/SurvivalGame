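; OceanWater is a water volume that switches the player into swim mode while its Box is overlapped.
; Begin and end overlap set SiwmMode on player 0's BP_SurvivalCharacter, without checking which actor caused the overlap.
; Both events also replace the FollowCamera post-process settings, shifting color temperature, tint and contrast for an underwater look and resetting them on exit.
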(event `self.Box.OnComponentBeginOverlap`
  (params (OverlappedComponent :type "PrimitiveComponent Object Reference") (OtherActor :type "Actor Object Reference") (OtherComp :type "PrimitiveComponent Object Reference") (OtherBodyIndex :type Integer) (bFromSweep :type Boolean) (SweepResult :type "HitResult Structure (by ref)"))
  (bind _asbp_survival_character (cast `/Game/character/ThirdPersonBP/Blueprints/BP_SurvivalCharacter` (`GameplayStatics.GetPlayerCharacter` 0)))
  (set `/Game/character/ThirdPersonBP/Blueprints/BP_SurvivalCharacter.SiwmMode` true _asbp_survival_character)
  (set `CameraComponent.PostProcessSettings` (make `PostProcessSettings` :`WhiteTemp` 1500.0 :`WhiteTint` -0.1 :`ColorContrast` (`KismetMathLibrary.MakeVector4` 0.55724 0.589256 0.79 0.6)) (`/Game/character/ThirdPersonBP/Blueprints/BP_SurvivalCharacter.FollowCamera` _asbp_survival_character)))

(event `self.Box.OnComponentEndOverlap`
  (params (OverlappedComponent :type "PrimitiveComponent Object Reference") (OtherActor :type "Actor Object Reference") (OtherComp :type "PrimitiveComponent Object Reference") (OtherBodyIndex :type Integer))
  (bind _asbp_survival_character (cast `/Game/character/ThirdPersonBP/Blueprints/BP_SurvivalCharacter` (`GameplayStatics.GetPlayerCharacter` 0)))
  (set `/Game/character/ThirdPersonBP/Blueprints/BP_SurvivalCharacter.SiwmMode` false _asbp_survival_character)
  (set `CameraComponent.PostProcessSettings` (make `PostProcessSettings` :`ColorContrast` (`KismetMathLibrary.MakeVector4` 1.0 1.0 1.0 1.0)) (`/Game/character/ThirdPersonBP/Blueprints/BP_SurvivalCharacter.FollowCamera` _asbp_survival_character)))

(fn `UserConstructionScript`)