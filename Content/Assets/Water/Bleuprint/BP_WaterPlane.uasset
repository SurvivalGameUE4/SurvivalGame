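; BP_WaterPlane is a placeable water surface built as a grid of instanced plane meshes, sized by a Counter X/Y tile count.
; The construction script clears the WaterPlane instances, then adds one per cell, spaced by the mesh's own bounds so tiles sit edge to edge.
; It then offsets the instanced component to center the grid on the actor's origin.
; It has no runtime logic, as all event graph nodes are disabled.
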(fn `UserConstructionScript`
  (locals (X :type Integer) (Y :type Integer))
  (bind _waterplane (`self.WaterPlane`))
  (bind (_counter_x _counter_y) (`KismetMathLibrary.BreakVector2D` (`self.Counter`)))
  (bind (_counter_x_2 _counter_y_2) (`KismetMathLibrary.BreakVector2D` (`self.Counter`)))
  (`InstancedStaticMeshComponent.ClearInstances` (`self.WaterPlane`))
  (for _index (range (`KismetMathLibrary.FFloor` _counter_x))
    (set `local.X` _index)
    (for _index_2 (range (`KismetMathLibrary.FFloor` _counter_y))
      (set `local.Y` _index_2)
      (`InstancedStaticMeshComponent.AddInstance` (`self.WaterPlane`) (`KismetMathLibrary.MakeTransform` (`KismetMathLibrary.MakeVector` (* (`local.X`) (* (.x (`.Max` (`StaticMeshComponent.GetLocalBounds` (`self.WaterPlane`)))) 2.0)) (* (`local.Y`) (* (.y (`.Max` (`StaticMeshComponent.GetLocalBounds` (`self.WaterPlane`)))) 2.0)))))))
  (`SceneComponent.K2_SetRelativeLocation` _waterplane (`KismetMathLibrary.MakeVector` (- 0.0 (* (- (`KismetMathLibrary.FFloor` _counter_x_2) 1) (.x (`.Max` (`StaticMeshComponent.GetLocalBounds` _waterplane))))) (- 0.0 (* (- (`KismetMathLibrary.FFloor` _counter_y_2) 1) (.y (`.Max` (`StaticMeshComponent.GetLocalBounds` _waterplane)))))) false false))