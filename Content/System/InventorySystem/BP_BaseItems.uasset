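; Base Blueprint for world inventory items that a character picks up by interacting with them.
; Interaction checks the character for inventory space, falling back to AddSpaceInventory; on success it passes ItemInfo to PickUpMessage and destroys the actor.
; The construction script rebuilds the ItemInfo struct with the actor's own class, so each item records its class alongside its type, stats and stacking data.
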(event `/Game/System/InventorySystem/Data/InteractData/BPI_Interact.Interaction`
  (params (Character :type "/Game/character/ThirdPersonBP/Blueprints/BP_SurvivalCharacter Object Reference"))
  (if (`/Game/character/ThirdPersonBP/Blueprints/BP_SurvivalCharacter.HasSpaceInventory` Character)
    (message `/Game/System/InventorySystem/Data/InteractData/BPI_Interact.PickUp` Character (`self.ItemInfo`) :!label _label)
    (`self.K2_DestroyActor`)
    (elif (`/Game/character/ThirdPersonBP/Blueprints/BP_SurvivalCharacter.AddSpaceInventory` Character)
      (goto _label))))

(fn `UserConstructionScript`
  (bind (_iteminfo_itemtype _iteminfo_equipmentslot _iteminfo_itemname _iteminfo_itemicon _iteminfo_itemdescription _iteminfo_itemclass _iteminfo_itemindex _iteminfo_healthpoints _iteminfo_hungerpoints _iteminfo_thirstpoints _iteminfo_warmer _iteminfo_cooler _iteminfo_durability _iteminfo_isstackable_ _iteminfo_maxstack _iteminfo_currentquantity _iteminfo_quantity) (break `/Game/System/InventorySystem/Data/S_ItemsInfo` (`self.ItemInfo`)))
  (`parent.UserConstructionScript`)
  (set `self.ItemInfo` (make `/Game/System/InventorySystem/Data/S_ItemsInfo` _iteminfo_itemtype _iteminfo_equipmentslot _iteminfo_itemname _iteminfo_itemicon _iteminfo_itemdescription (`GameplayStatics.GetObjectClass` self) _iteminfo_itemindex _iteminfo_healthpoints _iteminfo_hungerpoints _iteminfo_thirstpoints _iteminfo_warmer _iteminfo_cooler _iteminfo_durability _iteminfo_isstackable_ _iteminfo_maxstack _iteminfo_currentquantity _iteminfo_quantity)))